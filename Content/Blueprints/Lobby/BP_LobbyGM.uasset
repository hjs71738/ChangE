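; Lobby game mode that tracks connected players and their ready states, then moves the session to TopDownMap.
; Authority-side login and logout maintain parallel controller, info and ready arrays, reindexing players on exit.
; Changes are pushed to every BP_LobbyPC, and the kick list is rebuilt on player 0's lobby widget.
; When the ready count equals MaxPlayers, it shows loading screens, runs servertravel and updates the session.
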(event `LaunchTheGame`
  ;[1 1 1] 게임 실행
  (`KismetSystemLibrary.ExecuteConsoleCommand` "servertravel /Game/Maps/TopDownMap" (`GameplayStatics.GetPlayerController` 0))
  (bind _asgame_info_instance (cast `/Game/Blueprints/PlayerInfo/GameInfoInstance` (`GameplayStatics.GetGameInstance`)))
  (bind _extrasettings (`AdvancedSessionsLibrary.GetExtraSettings` (`/Game/Blueprints/PlayerInfo/GameInfoInstance.CurrentSession` _asgame_info_instance)))
  (`UpdateSessionCallbackProxyAdvanced.UpdateSession` _extrasettings (`/Game/Blueprints/PlayerInfo/GameInfoInstance.MaxPlayers` _asgame_info_instance)))

(event `self.K2_PostLogin`
  (params (NewPlayer :type "PlayerController Object Reference"))
  ;[1 1 1] 로그인 이후
  (`/Engine/EditorBlueprintResources/ActorMacros.Switch Has Authority`
    (:`Authority`
      (bind _returnvalue (`KismetArrayLibrary.Array_Add` (`self.AllPlayerControllers`) NewPlayer))
      (set `/Game/Blueprints/Lobby/BP_LobbyPC.PlayerIndex` _returnvalue (cast `/Game/Blueprints/Lobby/BP_LobbyPC` NewPlayer :!pure true))
      (`KismetArrayLibrary.Array_Add` (`self.ReadyPlayers`))
      (bind _asgame_info_instance (cast `/Game/Blueprints/PlayerInfo/GameInfoInstance` (`GameplayStatics.GetGameInstance`)))
      (set `self.MaxPlayers` (`/Game/Blueprints/PlayerInfo/GameInfoInstance.MaxPlayers` _asgame_info_instance))
      (bind _asbp_lobby_pc (cast `/Game/Blueprints/Lobby/BP_LobbyPC` NewPlayer))
      (`/Game/Blueprints/Lobby/BP_LobbyPC.LoadSavedFile` _asbp_lobby_pc)
      (`/Game/Blueprints/Lobby/BP_LobbyPC.SetUpLobbyMenu` _asbp_lobby_pc)
      (`self.EveryOneUpdate`))))

(event `EveryOneUpdate`
  (bind _allplayercontrollers (`self.AllPlayerControllers`))
  ;[1 1 1] 플레이어 접속/종료시 로비 화면 업데이트
  (bind _output_get (set `self.CurrentPlayers` (`KismetArrayLibrary.Array_Length` (`self.AllPlayerControllers`))))
  (if (> _output_get 0)
    (`KismetArrayLibrary.Array_Clear` (`self.ConnectedPlayers`))
    (for _array_element _allplayercontrollers
      (bind _asbp_lobby_pc (cast `/Game/Blueprints/Lobby/BP_LobbyPC` _array_element))
      (`KismetArrayLibrary.Array_Add` (`self.ConnectedPlayers`) (`/Game/Blueprints/Lobby/BP_LobbyPC.SPlayerInfo` _asbp_lobby_pc))
      (`/Game/Blueprints/Lobby/BP_LobbyPC.UpdateNumberOfPlayers` _asbp_lobby_pc (`self.CurrentPlayers`) (`self.MaxPlayers`)))
    (for _array_element_2 _allplayercontrollers
      (bind _asbp_lobby_pc_2 (cast `/Game/Blueprints/Lobby/BP_LobbyPC` _array_element_2))
      (`/Game/Blueprints/Lobby/BP_LobbyPC.AddPlayerInfo` _asbp_lobby_pc_2 (`self.ConnectedPlayers`) (`self.ReadyPlayers`)))
    (`self.UpdateKickList`)))

(event `self.K2_OnLogout`
  (params (ExitingController :type "Controller Object Reference"))
  (bind _allplayercontrollers (`self.AllPlayerControllers`))
  ;[1 1 1] 로그아웃시
  (for (_array_element _array_index) _allplayercontrollers
    (if (== ExitingController _array_element)
      (set `self.ExitingPlayerIndex` _array_index)
      (break)))
  (`KismetArrayLibrary.Array_Remove` (`self.AllPlayerControllers`) _array_index)
  (`KismetArrayLibrary.Array_Remove` (`self.ConnectedPlayers`) _array_index)
  (`KismetArrayLibrary.Array_Remove` (`self.ReadyPlayers`) _array_index)
  (for _array_element_2 _allplayercontrollers
    (bind _asbp_lobby_pc (cast `/Game/Blueprints/Lobby/BP_LobbyPC` _array_element_2))
    (bind _playerindex (`/Game/Blueprints/Lobby/BP_LobbyPC.PlayerIndex` _asbp_lobby_pc))
    (if (> _playerindex (`self.ExitingPlayerIndex`))
      (set `/Game/Blueprints/Lobby/BP_LobbyPC.PlayerIndex` (- _playerindex 1) _asbp_lobby_pc)))
  (`self.EveryOneUpdate`)
  (`self.UpdateKickList`))

(event `EveryOneReadyUpdate`
  ;[1 1 1] 코멘트
  (if (== (`self.ReadyPlayersCount`) (`self.MaxPlayers`))
    (for _array_element (`self.AllPlayerControllers`)
      (bind _asbp_lobby_pc (cast `/Game/Blueprints/Lobby/BP_LobbyPC` _array_element))
      (`/Game/Blueprints/Lobby/BP_LobbyPC.ShowLoadingScreen` _asbp_lobby_pc))
    (`self.LaunchTheGame`)
    (else
      (for _array_element_2 (`self.AllPlayerControllers`)
        (bind _asbp_lobby_pc_2 (cast `/Game/Blueprints/Lobby/BP_LobbyPC` _array_element_2))
        (`/Game/Blueprints/Lobby/BP_LobbyPC.ChangeReady` _asbp_lobby_pc_2 (`self.ReadyPlayers`))))))

(event `UpdateKickList`
  (bind _asbp_lobby_pc (cast `/Game/Blueprints/Lobby/BP_LobbyPC` (`GameplayStatics.GetPlayerController` 0) :!pure true))
  (bind _lobbymenuwb (`/Game/Blueprints/Lobby/BP_LobbyPC.LobbyMenuWB` _asbp_lobby_pc))
  ;[1 1 1] 강퇴 버튼 업데이트
  (`/Game/Blueprints/Lobby/UMG_Lobby.ClearKickList` _lobbymenuwb)
  (for _array_element (`self.AllPlayerControllers`)
    (if (== _array_element _asbp_lobby_pc)
      (`/Game/Blueprints/Lobby/UMG_Lobby.PassServer` _lobbymenuwb)
      (else
        (`/Game/Blueprints/Lobby/UMG_Lobby.MakeKickList` _lobbymenuwb _array_element)))))

(fn `UserConstructionScript`)