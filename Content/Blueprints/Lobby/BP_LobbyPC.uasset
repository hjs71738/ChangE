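; Lobby player controller that manages each player's lobby menu, ready state and saved player info.
; It creates UMG_Lobby and refreshes its player count, player list and ready list, later swapping it for a loading screen.
; The menu's ready dispatcher triggers RunOnServer, which toggles readiness and updates BP_LobbyGM's count and array.
; Player info persists through BP_PlayerSaveGame, while kicks and lost connections destroy the session and open MainMenu.
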(event `RunOnServer`
  (bind _asbp_lobby_gm (cast `/Game/Blueprints/Lobby/BP_LobbyGM` (`GameplayStatics.GetGameMode`) :!pure true))
  ;[1 1 1] 레디
  (if (`self.IsReady`)
    (set `self.IsReady` false)
    (set `/Game/Blueprints/Lobby/BP_LobbyGM.ReadyPlayersCount` (- (`/Game/Blueprints/Lobby/BP_LobbyGM.ReadyPlayersCount` _asbp_lobby_gm) 1) _asbp_lobby_gm)
    (else
      (set `self.IsReady` true)
      (set `/Game/Blueprints/Lobby/BP_LobbyGM.ReadyPlayersCount` (+ (`/Game/Blueprints/Lobby/BP_LobbyGM.ReadyPlayersCount` _asbp_lobby_gm) 1) _asbp_lobby_gm)))
  (`KismetArrayLibrary.Array_Set` (`/Game/Blueprints/Lobby/BP_LobbyGM.ReadyPlayers` _asbp_lobby_gm) (`self.PlayerIndex`) (`self.IsReady`))
  (`/Game/Blueprints/Lobby/BP_LobbyGM.EveryOneReadyUpdate` _asbp_lobby_gm))

(event `self.ReceiveBeginPlay`
  ;[1 1 1] 코멘트
  (add `/Game/Blueprints/Lobby/UMG_Lobby.OnPlayerChangeReady` (`self.LobbyMenuWB`) (delegate `OnPlayerChangeReady`)))

(event `OnPlayerChangeReady`
  ;[1 1 1] 코멘트
  (`self.RunOnServer`))

(event `UpdateSaveFile`
  (bind _playersavegameref (`self.PlayerSaveGameRef`))
  ;[1 1 1] 플레이어 정보 저장(로비에서 또 인게임으로 넘어가야 하니까) 사용 안함
  (`/Engine/EditorBlueprintResources/StandardMacros.IsValid` (`self.PlayerSaveGameRef`)
    (:`Is Valid`
      _)
    (:`Is Not Valid`
      (bind _returnvalue (`GameplayStatics.CreateSaveGameObject` "/Game/Blueprints/PlayerInfo/BP_PlayerSaveGame.BP_PlayerSaveGame_C"))
      (set `self.PlayerSaveGameRef` _returnvalue)))
  (set `/Game/Blueprints/PlayerInfo/BP_PlayerSaveGame.S_PlayerInfo` (`self.SPlayerInfo`) _playersavegameref)
  (`GameplayStatics.SaveGameToSlot` _playersavegameref (`self.PlayerSettingsSave`)))

(event `LoadSavedFile`
  ;[1 1 1] 코멘트
  (`GameplayStatics.DoesSaveGameExist` (`self.PlayerSettingsSave`))
  (`self.LoadGame`))

(event `SetUpLobbyMenu`
  ;[1 1 1] 메뉴 표시
  (set `self.bShowMouseCursor` true)
  (bind _returnvalue (`|CreateWidget` "/Game/Blueprints/Lobby/UMG_Lobby.UMG_Lobby_C" (`GameplayStatics.GetPlayerController` 0)))
  (bind _output_get (set `self.LobbyMenuWB` _returnvalue))
  (`UserWidget.AddToViewport` _output_get 0)
  (`WidgetBlueprintLibrary.SetInputMode_UIOnlyEx` self _output_get))

(event `UpdateNumberOfPlayers`
  (params (CurrentPlayers :type Integer) (MaxPlayers :type Integer))
  (bind _lobbymenuwb (`self.LobbyMenuWB`))
  ;[1 1 1] 접속 플레이어 수 표시
  (`/Engine/EditorBlueprintResources/StandardMacros.IsValid` _lobbymenuwb
    (:`Is Valid`
      (set `/Game/Blueprints/Lobby/UMG_Lobby.PlayerDisplay` (`|FormatText` "{CurrentPlayers} / {MaxPlayers}" (`KismetTextLibrary.Conv_IntToText` CurrentPlayers) (`KismetTextLibrary.Conv_IntToText` MaxPlayers)) _lobbymenuwb))))

(event `AddPlayerInfo`
  (params (ConnectedPlayerInfo :type "Array of /Game/Blueprints/PlayerInfo/PlayerInfo Structure") (PlayersReadyInfo :type "Array of Boolean"))
  (bind _lobbymenuwb (`self.LobbyMenuWB`))
  ;[1 1 1] 플레이어 리스트 추가하고 로비 업데이트
  (bind _output_get (set `self.Connected Players` ConnectedPlayerInfo))
  (`/Engine/EditorBlueprintResources/StandardMacros.IsValid` _lobbymenuwb
    (:`Is Valid`
      (`/Game/Blueprints/Lobby/UMG_Lobby.ClearPlayerList` _lobbymenuwb)
      (`/Game/Blueprints/Lobby/UMG_Lobby.ClearPlayerReadyList` _lobbymenuwb)
      (for _array_element _output_get
        (`/Game/Blueprints/Lobby/UMG_Lobby.UpdateLobbyPlayerInfo` _lobbymenuwb _array_element))
      (`self.ChangeReady` PlayersReadyInfo))))

(event `ShowLoadingScreen`
  ;[1 1 1] 로딩 스크린 불러오기
  (`Widget.RemoveFromParent` (`self.LobbyMenuWB`))
  (bind _returnvalue (`|CreateWidget` "/Game/Blueprints/Lobby/UMG_LoadingScreen.UMG_LoadingScreen_C" self))
  (`UserWidget.AddToViewport` _returnvalue 0))

(event `ChangeReady`
  (params (ReadyPlayers :type "Array of Boolean"))
  (bind _lobbymenuwb (`self.LobbyMenuWB`))
  ;[1 1 1] 코멘트
  (`/Game/Blueprints/Lobby/UMG_Lobby.ClearPlayerReadyList` _lobbymenuwb)
  (for _array_element ReadyPlayers
    (`/Game/Blueprints/Lobby/UMG_Lobby.UpdateLobbyReadyInfo` _lobbymenuwb _array_element)))

(event `ServerConnectionLost`
  ;[1 1 1] 코멘트
  (`DestroySessionCallbackProxy.DestroySession` self
    (:`OnSuccess`
      (`GameplayStatics.OpenLevel` "MainMenu"))))

(event `CheckIdEmpty`
  (bind _splayerinfo_myplayername (break `/Game/Blueprints/PlayerInfo/PlayerInfo` (`self.SPlayerInfo`)))
  ;[1 1 1] Id 공백 여부 확인
  (if (`KismetTextLibrary.EqualEqual_TextText` _splayerinfo_myplayername (`KismetTextLibrary.Conv_StringToText` ""))
    (set `self.SPlayerInfo` (make `/Game/Blueprints/PlayerInfo/PlayerInfo` (`|FormatText` "Player{idx}" (`KismetStringLibrary.Conv_IntToString` (`self.PlayerIndex`)))))
    (`self.SaveGame`)))

(event `YouAreKicked`
  ;[1 1 1] 강퇴
  (`DestroySessionCallbackProxy.DestroySession` self
    (:`OnSuccess`
      (`GameplayStatics.OpenLevel` "MainMenu"))))

(fn `LoadGame`
  (bind _returnvalue (`GameplayStatics.LoadGameFromSlot` (`self.PlayerSettingsSave`)))
  (bind _asbp_player_save_game (cast `/Game/Blueprints/PlayerInfo/BP_PlayerSaveGame` _returnvalue))
  (setmembers `/Game/Blueprints/PlayerInfo/PlayerInfo` :`StructRef` (`self.SPlayerInfo`) :`MyPlayerName` (`.MyPlayerName_2_17EBB7494872605B06D1C7869EBF5D65` (break `/Game/Blueprints/PlayerInfo/PlayerInfo` (`/Game/Blueprints/PlayerInfo/BP_PlayerSaveGame.S_PlayerInfo` _asbp_player_save_game)))))

(fn `SaveGame`
  (bind _playersavegameref (`self.PlayerSaveGameRef`))
  (`/Engine/EditorBlueprintResources/StandardMacros.IsValid` (`self.PlayerSaveGameRef`)
    (:`Is Valid`
      _)
    (:`Is Not Valid`
      (bind _returnvalue (`GameplayStatics.CreateSaveGameObject` "/Game/Blueprints/PlayerInfo/BP_PlayerSaveGame.BP_PlayerSaveGame_C"))
      (set `self.PlayerSaveGameRef` _returnvalue)))
  (set `/Game/Blueprints/PlayerInfo/BP_PlayerSaveGame.S_PlayerInfo` (`self.SPlayerInfo`) _playersavegameref)
  (`GameplayStatics.SaveGameToSlot` _playersavegameref (`self.PlayerSettingsSave`)))

(fn `UserConstructionScript`)