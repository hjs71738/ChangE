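; Game instance that handles multiplayer sessions and front-end menus for the game.
; LaunchLobby creates an advanced session tagged with the server name and player cap, then opens Lobby as a listen server; JoinServer joins a supplied search result.
; Show events lazily create and cache widgets; both main menu and browser use UMG_ServerBrowser.
; DisplayErrorMessage is an empty stub, so join failures show nothing.
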(event `JoinServer`
  (params (SesionToJoin :type "BlueprintSessionResult Structure"))
  ;[1 1 1] 서버 접속
  (bind _output_get (set `self.CurrentSession` SesionToJoin))
  (`JoinSessionCallbackProxy.JoinSession` (`GameplayStatics.GetPlayerController` 0) _output_get
    (:`OnFailure`
      (`self.DisplayErrorMessage` "failed to join session"))))

(event `LaunchLobby`
  (params (NumberOfPlayers :type Integer) (ServerName :type Text))
  ;[1 1 1] 로비 열어줌(에러 메시지 창 만들어야 함)
  (bind _output_get (set `self.MaxPlayers` NumberOfPlayers))
  (`CreateSessionCallbackProxyAdvanced.CreateAdvancedSession` (`|MakeArray` (`AdvancedSessionsLibrary.MakeLiteralSessionPropertyString` "GAMENAME" (`KismetTextLibrary.Conv_TextToString` ServerName))) (`GameplayStatics.GetPlayerController` 0) _output_get
    (:`OnSuccess`
      (`GameplayStatics.OpenLevel` "Lobby" true "listen"))
    (:`OnFailure`
      (`KismetSystemLibrary.PrintString` "failed to create."))))

(event `ShowHostMenu`
  ;[1 1 1] 호스트 메뉴 열어줌
  (`/Engine/EditorBlueprintResources/StandardMacros.IsValid` (`self.HostMenuWB`)
    (:`Is Valid`
      _)
    (:`Is Not Valid`
      (bind _returnvalue (`|CreateWidget` "/Game/Blueprints/HostMenu/UMG_HostMenu.UMG_HostMenu_C" (`GameplayStatics.GetPlayerController` 0)))
      (set `self.HostMenuWB` _returnvalue)))
  (`UserWidget.AddToViewport` (`self.HostMenuWB`) 0))

(event `ShowMainMenu`
  (bind _returnvalue (`GameplayStatics.GetPlayerController` 0))
  ;[1 1 1] 메인 메뉴 보여줌
  (`/Engine/EditorBlueprintResources/StandardMacros.IsValid` (`self.MainMenuWB`)
    (:`Is Valid`
      _)
    (:`Is Not Valid`
      (bind _returnvalue_2 (`|CreateWidget` "/Game/Blueprints/ServerBroswer/UMG_ServerBrowser.UMG_ServerBrowser_C" _returnvalue))
      (set `self.MainMenuWB` _returnvalue_2)))
  (`UserWidget.AddToViewport` (`self.MainMenuWB`) 0)
  (set `PlayerController.bShowMouseCursor` true _returnvalue))

(event `ShowServerBrowserMenu`
  (bind _returnvalue (`GameplayStatics.GetPlayerController` 0))
  ;[1 1 1] 서버 브라우저 메뉴 보여줌
  (`/Engine/EditorBlueprintResources/StandardMacros.IsValid` (`self.ServerBrowserWB`)
    (:`Is Valid`
      _)
    (:`Is Not Valid`
      (bind _returnvalue_2 (`|CreateWidget` "/Game/Blueprints/ServerBroswer/UMG_ServerBrowser.UMG_ServerBrowser_C" _returnvalue))
      (bind _output_get (set `self.ServerBrowserWB` _returnvalue_2))))
  (`UserWidget.AddToViewport` _output_get 0)
  (set `PlayerController.bShowMouseCursor` true _returnvalue))