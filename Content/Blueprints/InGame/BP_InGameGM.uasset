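; In-game GameMode for a multiplayer flag-capture match, tracking player controllers, the flag and the player count.
; It respawns players at random PlayerStarts, attaches the captured flag to the carrier's mesh socket and pushes the owner's name to all players.
; Player clicks trigger a hit alarm and debuff.
; Logouts notify remaining players and end the game when one remains, with EndGame sending win or lose to each controller.
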(event `DetachFlagFromCharacter`
  (params (Player :type "/Game/Blueprints/InGame/BP_Player Object Reference"))
  (`SceneComponent.K2_DetachFromComponent` (`Character.Mesh` Player) "KeepRelative" "KeepWorld" "KeepWorld" false))

(event `SpawnPlayer`
  (params (PlayerController :type "PlayerController Object Reference"))
  (bind _returnvalue (`Controller.K2_GetPawn` PlayerController))
  (bind _startpositions (`self.StartPositions`))
  ;[1 0 0.6094] 코멘트
  (bind _outactors (`GameplayStatics.GetAllActorsOfClass` "/Script/Engine.PlayerStart"))
  (set `self.StartPositions` _outactors)
  (`/Engine/EditorBlueprintResources/StandardMacros.IsValid` _returnvalue
    (:`Is Valid`
      (`self.K2_DestroyActor` _returnvalue)
      (bind _returnvalue_2 (`|SpawnActorFromClass` "/Game/Blueprints/InGame/BP_Player.BP_Player_C" (`self.GetTransform` (`|GetArrayItem` _startpositions (`KismetMathLibrary.RandomIntegerInRange` 0 (- (`KismetArrayLibrary.Array_Length` _startpositions) 1)))) "Undefined" "MultiplyWithRoot" null null))
      (`Controller.Possess` PlayerController _returnvalue_2))))

(event `FlagCapturedAndNotifyAllPlayers`
  (params (WhoCaputre :type "/Game/Blueprints/InGame/BP_Player Object Reference"))
  (bind _playersettings_myplayername (break `/Game/Blueprints/PlayerInfo/PlayerInfo` (`/Game/Blueprints/InGame/BP_InGamePC.PlayerSettings` (cast `/Game/Blueprints/InGame/BP_InGamePC` (`Pawn.GetController` WhoCaputre) :!pure true))))
  ;[0.875 1 0] 코멘트
  (set `/Game/Blueprints/InGame/BP_Player.HasFlag?` true WhoCaputre)
  (bind _returnvalue (`self.K2_AttachToComponent` (`self.Flag`) (`Character.Mesh` WhoCaputre) "FlagSlot" "SnapToTarget" "KeepWorld" "KeepWorld" false))
  (if _returnvalue
    (for _array_element (`self.AllPlayerControllers`)
      (bind _asbp_in_game_pc (cast `/Game/Blueprints/InGame/BP_InGamePC` _array_element))
      (bind _asbp_player (cast `/Game/Blueprints/InGame/BP_Player` (`Controller.K2_GetPawn` _asbp_in_game_pc)))
      (set `/Game/Blueprints/InGame/BP_Player.HasFlag?` true _asbp_player)
      (`/Game/Blueprints/InGame/BP_Player.ChangeFlagOwnersName` _asbp_player _playersettings_myplayername))))

(event `self.K2_OnSwapPlayerControllers`
  (params (OldPC :type "PlayerController Object Reference") (NewPC :type "PlayerController Object Reference"))
  ;[1 0.4922 0] 코멘트
  (`KismetArrayLibrary.Array_Add` (`self.AllPlayerControllers`) NewPC)
  (`/Engine/EditorBlueprintResources/ActorMacros.Switch Has Authority`
    (:`Authority`
      (`/Game/Blueprints/InGame/BP_InGamePC.LoadSavedId` (cast `/Game/Blueprints/InGame/BP_InGamePC` NewPC :!pure true)))))

(event `self.ReceiveBeginPlay`
  ;[0 0.2031 1] 코멘트
  (bind _asgame_info_instance (cast `/Game/Blueprints/PlayerInfo/GameInfoInstance` (`GameplayStatics.GetGameInstance`)))
  (set `self.NumOfPlayers` (`/Game/Blueprints/PlayerInfo/GameInfoInstance.MaxPlayers` _asgame_info_instance))
  (bind _returnvalue (`GameplayStatics.GetActorOfClass` "/Game/Blueprints/InGame/BP_Flag.BP_Flag_C"))
  (set `self.Flag` _returnvalue))

(event `ClickOtherPlayer`
  (params (Player :type "/Game/Blueprints/InGame/BP_InGamePC Object Reference") (WhoAttack :type Text))
  ;[1 0.4688 0] 코멘트
  (`/Game/Blueprints/InGame/BP_InGamePC.GetHitAlram` Player WhoAttack)
  (if (not (`/Game/Blueprints/InGame/BP_InGamePC.IsInDebuffnow?` Player))
    (`/Game/Blueprints/InGame/BP_InGamePC.StartDebuff` Player)))

(event `self.K2_OnLogout`
  (params (ExitingController :type "Controller Object Reference"))
  (bind _allplayercontrollers (`self.AllPlayerControllers`))
  (bind _numofplayers (`self.NumOfPlayers`))
  ;[0.9219 0 1] 코멘트
  (`/Engine/EditorBlueprintResources/StandardMacros.DecrementInt` _numofplayers
    (:`  `
      (for (_array_element _array_index) _allplayercontrollers
        (if (== _array_element ExitingController)
          (`KismetArrayLibrary.Array_Remove` _allplayercontrollers _array_index)
          (for _array_element_2 _allplayercontrollers
            (bind _asbp_in_game_pc (cast `/Game/Blueprints/InGame/BP_InGamePC` _array_element_2))
            (`/Game/Blueprints/InGame/BP_InGamePC.NoticePlayerOut` _asbp_in_game_pc _numofplayers)
            (if (== 1 (`KismetArrayLibrary.Array_Length` (`self.AllPlayerControllers`)))
              (`self.EndGame` null))))))))

(event `DecreaseSpeed`
  (params (TargetMovement :type "CharacterMovementComponent Object Reference"))
  ;[0.4531 0 1] 코멘트
  (set `CharacterMovementComponent.MaxWalkSpeed` 50.0 TargetMovement))

(event `EndGame`
  (params (Player :type "/Game/Blueprints/InGame/BP_Player Object Reference"))
  ;[0.3359 0 1] 코멘트
  (set `/Game/Blueprints/InGame/BP_InGamePC.IsWinner` true (cast `/Game/Blueprints/InGame/BP_InGamePC` (`Pawn.GetController` Player) :!pure true))
  (for _array_element (`self.AllPlayerControllers`)
    (bind _asbp_in_game_pc (cast `/Game/Blueprints/InGame/BP_InGamePC` _array_element))
    (if (`/Game/Blueprints/InGame/BP_InGamePC.IsWinner` _asbp_in_game_pc)
      (`/Game/Blueprints/InGame/BP_InGamePC.GameWin` _asbp_in_game_pc)
      (else
        (`/Game/Blueprints/InGame/BP_InGamePC.GameLose` _asbp_in_game_pc)))))

(fn `UserConstructionScript`)