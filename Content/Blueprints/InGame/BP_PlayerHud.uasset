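; BP_PlayerHud toggles the in-game option menu on and off through its ShowOptionMenu event.
; The first call creates UMG_OptionMenu, adds it to the viewport and stores the passed key on it; later calls reuse that widget.
; Opening focuses the menu with UI-only input.
; Closing collapses it, restores game-only input with the mouse cursor shown and sets permanent mouse capture including the initial mouse down.
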(event `ShowOptionMenu`
  (params (Key :type "Key Structure" :default "None"))
  (bind _optionwidget (`self.OptionWidget`))
  (bind _optionwidget_2 (`self.OptionWidget`))
  (`/Engine/EditorBlueprintResources/StandardMacros.IsValid` (`self.OptionWidget`)
    (:`Is Valid`
      (if (`Widget.IsVisible` _optionwidget_2)
        (`self.CollapseWidget` _optionwidget_2)
        (`GameplayStatics.SetViewportMouseCaptureMode` "CapturePermanently_IncludingInitialMouseDown")
        (else
          (`Widget.SetVisibility` _optionwidget_2 "Visible")
          (`WidgetBlueprintLibrary.SetInputMode_UIOnlyEx` (`GameplayStatics.GetPlayerController` 0) _optionwidget :!label _label)
          (`Widget.SetKeyboardFocus` _optionwidget))))
    (:`Is Not Valid`
      (bind _returnvalue (`|CreateWidget` "/Game/Blueprints/InGame/UMG_OptionMenu.UMG_OptionMenu_C"))
      (bind _output_get (set `self.OptionWidget` _returnvalue))
      (`UserWidget.AddToViewport` _output_get 0)
      (set `/Game/Blueprints/InGame/UMG_OptionMenu.InputShowOption` Key _output_get)
      (goto _label))))

(fn `CollapseWidget`
  (params (OptionMenu :type "/Game/Blueprints/InGame/UMG_OptionMenu Object Reference"))
  (bind _returnvalue (`GameplayStatics.GetPlayerController` 0))
  (`/Engine/EditorBlueprintResources/StandardMacros.IsValid` OptionMenu
    (:`Is Valid`
      (`Widget.SetVisibility` OptionMenu "Collapsed"))
    (:`Is Not Valid`
      _))
  (`WidgetBlueprintLibrary.SetInputMode_GameOnly` _returnvalue)
  (set `PlayerController.bShowMouseCursor` true _returnvalue))

(fn `UserConstructionScript`)