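; In-game player controller for a multiplayer click-to-move game where players click each other's pawns to hit them.
; Clicking another pawn passes the hit to BP_InGameGM, while holding elsewhere runs a timer for cursor-driven movement, issued both locally and via server on clients.
; It also requests spawning from the game mode, loads the saved name, drives the debuff countdown UI, and shows exit and win/lose widgets before returning to MainMenu.
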(event `self.ReceiveBeginPlay`
  ;[0.05098 0.05098 0.05098] Add Mapping Context
  (if (`self.IsLocalController`)
    (`WidgetLayoutLibrary.RemoveAllWidgets`)
    (`WidgetBlueprintLibrary.SetInputMode_GameOnly` self)
    (`GameplayStatics.SetViewportMouseCaptureMode` "CapturePermanently_IncludingInitialMouseDown")
    (`self.Spawn`)))

(event `LoadSavedId`
  ;[0.6406 1 0] 메인 메뉴에서 만든 아이디 불러오기
  (bind _returnvalue (`GameplayStatics.LoadGameFromSlot` (`self.PlayerSettingsSave`)))
  (bind _asbp_player_save_game (cast `/Game/Blueprints/PlayerInfo/BP_PlayerSaveGame` _returnvalue))
  (set `self.PlayerSettings` (`/Game/Blueprints/PlayerInfo/BP_PlayerSaveGame.S_PlayerInfo` _asbp_player_save_game)))

(event `NoticePlayerOut`
  (params (NumOfLeftPlayers :type Integer))
  (bind _playersettings_myplayername (break `/Game/Blueprints/PlayerInfo/PlayerInfo` (`self.PlayerSettings`)))
  ;[0.5703 0 1] 플레이어 나감 알림
  (bind _returnvalue (`|CreateWidget` "/Game/Blueprints/InGame/UMG_PlayerOutAlarm.UMG_PlayerOutAlarm_C" (`GameplayStatics.GetPlayerController` 0) NumOfLeftPlayers _playersettings_myplayername))
  (`UserWidget.AddToViewport` _returnvalue 0)
  (`KismetSystemLibrary.Delay` 3.0)
  (`Widget.RemoveFromParent` _returnvalue))

(event `Spawn`
  ;[0 1 0.5547] 부활
  (bind _asbp_in_game_gm (cast `/Game/Blueprints/InGame/BP_InGameGM` (`GameplayStatics.GetGameMode`)))
  (`/Game/Blueprints/InGame/BP_InGameGM.SpawnPlayer` _asbp_in_game_gm self)
  (bind _asbp_player (cast `/Game/Blueprints/InGame/BP_Player` (`self.K2_GetPawn`)))
  (`/Game/Blueprints/InGame/BP_Player.SetupUi` _asbp_player))

(event `InputAction|SetDestination`
  (params (Key :type "Key Structure"))
  ;[0.2188 0 1] 코멘트
  (:`Pressed`
    (set `self.InputPressed` true)
    (bind _newparam (`self.Click Other Clients`))
    (if _newparam
      (`self.StopMovement`)
      (else
        (`self.StartClickTimer`))))
  (:`Released`
    (set `self.InputPressed` false)
    (`self.StopClickTimer`)))

(event `StartDebuff`
  ;[0 1 0.9063] 코멘트
  (set `self.IsInDebuffnow?` true)
  (bind _returnvalue (`KismetSystemLibrary.K2_SetTimerDelegate` (delegate `UpdateDebuffTime`) 1.0 true))
  (set `self.DebuffTimerHandle` _returnvalue))

(event `UpdateDebuffTimes`
  (params (LeftTime :type Integer))
  ;[1 0.3984 0] 코멘트
  (`/Game/Blueprints/InGame/UMG_PlayerUi.ChagneLeftTimesOfDebuff` (`/Game/Blueprints/InGame/BP_Player.UserUi` (cast `/Game/Blueprints/InGame/BP_Player` (`self.K2_GetPawn`) :!pure true)) LeftTime))

(event `UpdateDebuffTime`
  ;[0 1 0.9063] 코멘트
  (if (== 0 (`self.DebuffLeftTimes`))
    (`KismetSystemLibrary.K2_ClearAndInvalidateTimerHandle` (`self.DebuffTimerHandle`))
    (set `self.IsInDebuffnow?` false)
    (set `self.DebuffLeftTimes` 10)
    (else
      (bind _result (`/Engine/EditorBlueprintResources/StandardMacros.DecrementInt` (`self.DebuffLeftTimes`))
        (:`  `
          (bind _output_get (set `self.DebuffLeftTimes` _result))
          (`self.UpdateDebuffTimes` _output_get))))))

(event `WinOrLose`
  (params (WinOrNot :type Boolean) (WinnersName :type Text))
  (bind _returnvalue (`GameplayStatics.GetPlayerController` 0))
  ;[0.03125 1 0] 코멘트
  (bind _returnvalue_2 (`|CreateWidget` "/Game/Blueprints/InGame/UMG_WinOrLose.UMG_WinOrLose_C" _returnvalue WinOrNot))
  (`/Game/Blueprints/InGame/UMG_WinOrLose.ShowWinnerName` _returnvalue_2 WinnersName)
  (`/Game/Blueprints/InGame/UMG_WinOrLose.ShowResult` _returnvalue_2)
  (`UserWidget.AddToViewport` _returnvalue_2 0)
  (`KismetSystemLibrary.Delay` 3.0)
  (`DestroySessionCallbackProxy.DestroySession` _returnvalue
    (:`OnSuccess`
      (`GameplayStatics.OpenLevel` "MainMenu"))))

(event `StartClickTimer`
  ;[0.6875 1 0] 이동 판단 타이머 시작
  (bind _returnvalue (`KismetSystemLibrary.K2_SetTimerDelegate` (`|CreateDelegate` :!event `UpdateClickLocation`) 0.01 true))
  (set `self.ClickLocationTimerHandle` _returnvalue))

(event `Server_MoveToLocation`
  (params (Controller :type "Controller Object Reference") (Goal :type "Vector Structure (by ref)"))
  ;[0.07812 1 0] Move On Server
  (`AIBlueprintHelperLibrary.SimpleMoveToLocation` Controller Goal))

(event `SpawnMouseFxCursor`
  ;[0 1 0.0625] 코멘트
  (`NiagaraFunctionLibrary.SpawnSystemAtLocation` (`self.FXCursor`)))

(event `커스텀이벤트`
  ;[0 1 0.25] 질문
  (`KismetSystemLibrary.K2_SetTimerDelegate` (`|CreateDelegate` :!event `Why?`) 1.0 true))

(event `Why?`
  ;[0 1 0.25] 질문
  (if (not (== 0 (`self.DebuffLeftTimes`)))
    (bind _result (`/Engine/EditorBlueprintResources/StandardMacros.DecrementInt` (`self.DebuffLeftTimes`))
      (:`  `
        (bind _output_get (set `self.DebuffLeftTimes` _result))
        (`/Game/Blueprints/InGame/UMG_PlayerUi.ChagneLeftTimesOfDebuff` (`/Game/Blueprints/InGame/BP_Player.UserUi` (cast `/Game/Blueprints/InGame/BP_Player` (`self.K2_GetPawn`) :!pure true)) _output_get)))))

(event `UpdateClickLocation`
  ;[1 0.7734 0] 코멘트
  (`self.MoveToHitLocation` (`.Location` (`self.GetLocationUnderCursor`))))

(event `StopClickTimer`
  ;[1 0 0.3281] 이동판단 타이머 끄기
  (`KismetSystemLibrary.K2_ClearAndInvalidateTimerHandle` (`self.ClickLocationTimerHandle`)))

(event `InputAction|Options`
  (params (Key :type "Key Structure"))
  ;[1 0.7969 0] 코멘트
  (:`Pressed`
    (bind _asbp_player_hud (cast `/Game/Blueprints/InGame/BP_PlayerHud` (`self.GetHUD`)))
    (`/Game/Blueprints/InGame/BP_PlayerHud.ShowOptionMenu` _asbp_player_hud Key)))

(event `ClickOnServer`
  (params (Player :type "Actor Object Reference"))
  (bind _playersettings_myplayername (break `/Game/Blueprints/PlayerInfo/PlayerInfo` (`self.PlayerSettings`)))
  ;[1 0 0.3047] 코멘트
  (bind _asbp_player (cast `/Game/Blueprints/InGame/BP_Player` Player))
  (bind _asbp_in_game_pc (cast `/Game/Blueprints/InGame/BP_InGamePC` (`Pawn.GetController` _asbp_player)))
  (bind _playersettings_myplayername_2 (break `/Game/Blueprints/PlayerInfo/PlayerInfo` (`/Game/Blueprints/InGame/BP_InGamePC.PlayerSettings` _asbp_in_game_pc)))
  (`self.ChangeHitUserName` _playersettings_myplayername_2)
  (bind _asbp_in_game_gm (cast `/Game/Blueprints/InGame/BP_InGameGM` (`GameplayStatics.GetGameMode`)))
  (`/Game/Blueprints/InGame/BP_InGameGM.ClickOtherPlayer` _asbp_in_game_gm _asbp_in_game_pc _playersettings_myplayername))

(event `ChangeHitUserName`
  (params (PlayerName :type Text))
  (bind (_asbp_player _bsuccess) (cast `/Game/Blueprints/InGame/BP_Player` (`self.K2_GetPawn`) :!pure true))
  ;[0.7812 1 0] 코멘트
  (if _bsuccess
    (`TextBlock.SetText` (`/Game/Blueprints/InGame/UMG_PlayerUi.HitName` (`/Game/Blueprints/InGame/BP_Player.UserUi` _asbp_player)) PlayerName)))

(event `GetHitAlram`
  (params (WhoAttackYou :type Text))
  ;[1 0 0.3047] 코멘트
  (`KismetSystemLibrary.PrintString` (`KismetTextLibrary.Conv_TextToString` (`|FormatText` "You are hit by {name}!!" WhoAttackYou))))

(fn `Click Other Clients`
  (returns (NewParam :type Boolean))
  (bind _hitresult (`self.GetHitResultUnderCursorForObjects` (`|MakeArray` "ObjectTypeQuery3" :!type "EObjectTypeQuery Enum") false))
  (bind _playersettings_myplayername (break `/Game/Blueprints/PlayerInfo/PlayerInfo` (`/Game/Blueprints/InGame/BP_InGamePC.PlayerSettings` (cast `/Game/Blueprints/InGame/BP_InGamePC` (`Pawn.GetController` (cast `/Game/Blueprints/InGame/BP_Player` (`.HitActor` (`GameplayStatics.BreakHitResult` _hitresult)) :!pure true)) :!pure true))))
  ;[0.8516 1 0] 코멘트
  (if (and (`GameplayStatics.BreakHitResult` _hitresult) (!= (`.HitActor` (`GameplayStatics.BreakHitResult` _hitresult)) (`self.K2_GetPawn`)))
    (`KismetSystemLibrary.PrintText` _playersettings_myplayername)
    (`self.ClickOnServer` (`.HitActor` (`GameplayStatics.BreakHitResult` _hitresult)))
    (return true)
    (else
      (return false))))

(fn `Follow`
  (params (Location :type "Vector Structure"))
  (bind _returnvalue (`self.K2_GetPawn`))
  (`Pawn.AddMovementInput` _returnvalue (`KismetMathLibrary.GetDirectionUnitVector` (`self.K2_GetActorLocation` _returnvalue) Location) 1.0 false))

(fn `GetLocationUnderCursor`
  (returns (Hit :type Boolean) (Location :type "Vector Structure"))
  (bind (_bblockinghit _binitialoverlap _time _distance _location) (`GameplayStatics.BreakHitResult` (`self.GetHitResultUnderCursorByChannel` "TraceTypeQuery1")))
  (return _bblockinghit _location))

(fn `GetLocationUnderFinger`
  (returns (Hit :type Boolean) (Location :type "Vector Structure"))
  (bind (_bblockinghit _binitialoverlap _time _distance _location) (`GameplayStatics.BreakHitResult` (`self.GetHitResultUnderFingerByChannel` "Touch1" "TraceTypeQuery1" false)))
  (return _bblockinghit _location))

(fn `MoveToHitLocation`
  (params (Location :type "Vector Structure"))
  (bind _location (`local.Location`))
  (`/Engine/EditorBlueprintResources/ActorMacros.Switch Has Authority`
    (:`Authority`
      (`self.Server_MoveToLocation` self self _location))
    (:`Remote`
      (`self.Server_MoveToLocation` self self _location)
      ;[1 1 1] 따로 리플리케이션 하는것? 소유 클라이언트에서 실행?
      (`AIBlueprintHelperLibrary.SimpleMoveToLocation` self (`local.Location`)))))

(fn `UserConstructionScript`)